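; BP_Statue_Judge is a rotatable puzzle statue that reports to a Sinner actor when it reaches its correct orientation.
; Overlap opens a gate for IA_Interact, and a DoOnce limits input to one 90-degree step at a time.
; A timeline lerps the rotation with sound, also at BeginPlay, then checks the position.
; Position 0 plays a success sound, updates the Sinner and leaves the statue locked; others re-arm interaction.
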(event Custom|UpdatePosition
  ;[0.1765 0.09804 0.09804 1 14] Para contabilizar el nº de giros (0º - 90º - 180º - 270º - 0º)
  (bind _result (Math|Integer|IncrementInt (Variables|Default|GetPosition))
    (:%20%20
      (if (> _result 3)
        (Variables|Default|SetPosition 0))
      (CallFunction|ActivateAnimation))))

(event Custom|CheckPosition
  ;[0.1765 0.09804 0.09804 1 14] Cuando esté en la POS correcta, -1
  (if (== (Variables|Default|GetPosition) 0)
    (Audio|PlaySoundatLocation "/Game/MyAssets/Statues/Sound/statue_correctposition.statue_correctposition" (Transformation|GetActorLocation) "0, 0, 0" 1.0 1.0 0.0 0 0 0 0)
    (Utilities|FlowControl|Delay 1.0)
    (Default|UpdatePuzzle (Variables|Default|GetSinner))
    (else
      (CallFunction|InteractReset))))

(event Custom|InteractReset
  (Utilities|FlowControl|DoOnce false) ; enters at Reset
)

(event Custom|ActivateAnimation
  (Variables|Default|SetStartRotation (Variables|Default|GetEndRotation))
  (Variables|Default|SetEndRotation (Math|Rotator|MakeRotator 0.0 0.0 (* (Variables|Default|GetPosition) 9e+01)))
  (Audio|PlaySoundatLocation "/Game/MyAssets/Statues/Sound/statue_rotate.statue_rotate" (Transformation|GetActorLocation) "0, 0, 0" 1.0 1.0 0.0 0 0 0 0)
  ;[0.3073 0.3073 0.1831 1 14] La animación del valor de la rotación
  (bind _alpha (Timeline|RotationAnimation PlayFromStart)
    (:Update
      ;[0.02843 0.06663 0.0999 1 12] Se aplicará la rotación deseada
      (Transformation|SetRelativeRotation (Variables|Default|GetStatue_Judge) (Math|Rotator|Lerp(Rotator) (Variables|Default|GetStartRotation) (Variables|Default|GetEndRotation) _alpha true) false false))
    (:Finished
      ;[1 1 1 1 12] Cuando termine la animación ver si -1 estatuas en el sinner
      (CallFunction|CheckPosition))))

(event Input|EnhancedActionEvents|EnhancedInputActionIA_Interact
  (params (ActionValue :type Boolean) (ElapsedSeconds :type Float%20%28double-precision%29) (TriggeredSeconds :type Float%20%28double-precision%29) (InputAction :type Input%20Action%20Object%20Reference :default "/Game/ThirdPerson/Input/Actions/IA_Interact.IA_Interact"))
  ;[0.1875 0.1875 0.1875] Sistema de interacción
  (:Started
    ;;[0.3125 0.3125 0.3125 1 14] No deja que pueda seguir el curso de los nodos a menos que...
    (Utilities|FlowControl|Gate true
      (:Exit
        (Utilities|FlowControl|DoOnce false
          (:Completed
            (CallFunction|UpdatePosition)))))))

(event EventBeginPlay
  ;[0.1875 0.1875 0.1875] Sistema de interacción
  (Input|EnableInput (Game|GetPlayerController 0))
  (CallFunction|ActivateAnimation))

(event Collision|EventActorBeginOverlap
  (params (OtherActor :type Actor%20Object%20Reference))
  ;[0.1875 0.1875 0.1875] Sistema de interacción
  ;;[0.349 0.1765 0.1765 1 14] SI PJ esté encima del obj se ABRE
  ;;[0.3125 0.3125 0.3125 1 14] No deja que pueda seguir el curso de los nodos a menos que...
  (Utilities|FlowControl|Gate true) ; enters at Open
)

(event EventTick
  (params (DeltaSeconds :type Float%20%28single-precision%29))
  ;[0.1875 0.1875 0.1875] Sistema de interacción
)

(event Collision|EventActorEndOverlap
  (params (OtherActor :type Actor%20Object%20Reference))
  ;[0.1875 0.1875 0.1875] Sistema de interacción
  ;;[0.349 0.2603 0.1423 1 14] Cuando el PJ deje de estar encima del obj se CIERRA
  ;;[0.3125 0.3125 0.3125 1 14] No deja que pueda seguir el curso de los nodos a menos que...
  (Utilities|FlowControl|Gate true) ; enters at Close
)

(fn ConstructionScript)