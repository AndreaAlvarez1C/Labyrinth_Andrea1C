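; BP_LeverFinal is an interactable lever that notifies the final door when pulled.
; It enables input for player controller 0 on BeginPlay, and a Gate lets IA_Interact through only between actor begin and end overlap events, with no check on the overlapping actor.
; The LeverRotation timeline lerps the lever mesh's relative rotation, then calls FinalDoorUpdate on the FinalDoor reference when finished.
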(event Input|EnhancedActionEvents|EnhancedInputActionIA_Interact
  (params (ActionValue :type Boolean) (ElapsedSeconds :type Float%20%28double-precision%29) (TriggeredSeconds :type Float%20%28double-precision%29) (InputAction :type Input%20Action%20Object%20Reference :default "/Game/ThirdPerson/Input/Actions/IA_Interact.IA_Interact"))
  ;[0.1875 0.1875 0.1875] Sistema de interacción
  (:Started
    ;;[0.3125 0.3125 0.3125 1 14] No deja que pueda seguir el curso de los nodos a menos que...
    (Utilities|FlowControl|Gate true
      (:Exit
        (bind _alpha (Timeline|LeverRotation Play)
          (:Update
            (Transformation|SetRelativeRotation (Variables|Default|GetLever_Lever) (Math|Rotator|Lerp(Rotator) "0.000000,90.000000,0.000000" "0.000000,90.000000,120.000000" _alpha) false false))
          (:Finished
            (Default|FinalDoorUpdate (Variables|Default|GetFinalDoor))))))))

(event EventBeginPlay
  ;[0.1875 0.1875 0.1875] Sistema de interacción
  (Input|EnableInput (Game|GetPlayerController 0)))

(event Collision|EventActorBeginOverlap
  (params (OtherActor :type Actor%20Object%20Reference))
  ;[0.1875 0.1875 0.1875] Sistema de interacción
  ;;[0.349 0.1765 0.1765 1 14] SI PJ esté encima del obj se ABRE
  ;;[0.3125 0.3125 0.3125 1 14] No deja que pueda seguir el curso de los nodos a menos que...
  (Utilities|FlowControl|Gate true) ; enters at Open
)

(event EventTick
  (params (DeltaSeconds :type Float%20%28single-precision%29))
  ;[0.1875 0.1875 0.1875] Sistema de interacción
)

(event Collision|EventActorEndOverlap
  (params (OtherActor :type Actor%20Object%20Reference))
  ;[0.1875 0.1875 0.1875] Sistema de interacción
  ;;[0.349 0.1765 0.1765 1 14] Cuando el PJ deje de estar encima del obj se CIERRA
  ;;[0.3125 0.3125 0.3125 1 14] No deja que pueda seguir el curso de los nodos a menos que...
  (Utilities|FlowControl|Gate true) ; enters at Close
)

(fn ConstructionScript)