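; Interactable hinged door that the player opens and closes with IA_Interact while overlapping it, optionally locked behind a key.
; A Gate driven by actor overlap filters the input; a locked door consumes one key from the cached BP_ThirdPersonCharacter or prints a warning.
; OpenCloseDoor uses a FlipFlop to play or reverse the DoorRotation timeline, lerping the mesh's relative rotation toward a swing direction set at BeginPlay by InvertDirection.
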(event Custom|OpenCloseDoor
  ;[0.03125 0.03125 0.03125] Abrir/Cerrar la puerta
  ;;[0.2708 0.2708 0.2708 1 14] Para poder abrir y cerrar la puerta
  (Utilities|FlowControl|FlipFlop
    (:A
      ;;[0.4688 0.4436 0.249 1 14] La variación de ALPHA en 0.7s
      (bind _alpha (Timeline|DoorRotation Play)
        (:Update
          (Transformation|SetRelativeRotation (Variables|Default|GetDoor_Door_GEO) (Math|Rotator|Lerp(Rotator) "0, 0, 0" (Variables|Default|GetDoorDirection) _alpha) false false))))
    (:B
      (Timeline|DoorRotation Reverse))))

(event Input|EnhancedActionEvents|EnhancedInputActionIA_Interact
  (params (ActionValue :type Boolean) (ElapsedSeconds :type Float%20%28double-precision%29) (TriggeredSeconds :type Float%20%28double-precision%29) (InputAction :type Input%20Action%20Object%20Reference :default "/Game/ThirdPerson/Input/Actions/IA_Interact.IA_Interact"))
  ;[0.1875 0.1875 0.1875] Sistema de interacción
  (:Started
    ;;[0.3125 0.3125 0.3125 1 14] No deja que pueda seguir el curso de los nodos a menos que...
    (Utilities|FlowControl|Gate true
      (:Exit
        ;[0.03125 0.03125 0.03125] Puerta cerrada/abierta
        (if (Variables|Default|GetisLocked)
          ;[0.1146 0.1146 0.1146] Para decidir si se puede abrir la puerta o no
          ;;[0.1823 0.05367 0.04937 1 14] SI está CERRADA
          (if (>= (Variables|/Game/ThirdPerson/Blueprints/BP_ThirdPersonCharacter.BP_ThirdPersonCharacter_C|GetKeys (Variables|Default|GetCharacter)) 1)
            ;;[0.2708 0.1608 0.1608 1 14] Ya no está cerrada
            (Variables|Default|SetisLocked false)
            ;;[0.04842 0.1094 0.08247 1 12] -1 llave
            (Math|Integer|DecrementInt (Variables|/Game/ThirdPerson/Blueprints/BP_ThirdPersonCharacter.BP_ThirdPersonCharacter_C|GetKeys (Variables|Default|GetCharacter))
              (:%20%20
                (CallFunction|OpenCloseDoor :!label _label)))
            (else
              (Development|PrintString "You need a key." true true "(R=0.046875,G=0.006878,B=0.006348,A=1.000000)")))
          (else
            (goto _label)))))))

(event EventBeginPlay
  ;[0.1875 0.1875 0.1875] Sistema de interacción
  (Input|EnableInput (Game|GetPlayerController 0))
  ;[0.1074 0.224 0.1853 1 14] Para no tener que referencias constantemente al Player
  (bind _asbp_third_person_character (Utilities|Casting|CastToBP_ThirdPersonCharacter (Game|GetPlayerCharacter 0)))
  (Variables|Default|SetCharacter _asbp_third_person_character)
  ;[0.125 0.07878 0.07878 1 14] Rotación interna/externa de la puerta
  (if (Variables|Default|GetInvertDirection)
    (Variables|Default|SetDoorDirection "0.000000,90.000000,0.000000")
    (else
      (Variables|Default|SetDoorDirection "0.000000,-90.000000,0.000000"))))

(event Collision|EventActorBeginOverlap
  (params (OtherActor :type Actor%20Object%20Reference))
  ;[0.1875 0.1875 0.1875] Sistema de interacción
  ;;[0.349 0.1765 0.1765 1 14] SI PJ esté encima del obj se ABRE
  ;;[0.3125 0.3125 0.3125 1 14] No deja que pueda seguir el curso de los nodos a menos que...
  (Utilities|FlowControl|Gate true) ; enters at Open
)

(event EventTick
  (params (DeltaSeconds :type Float%20%28single-precision%29))
  ;[0.1875 0.1875 0.1875] Sistema de interacción
)

(event Collision|EventActorEndOverlap
  (params (OtherActor :type Actor%20Object%20Reference))
  ;[0.1875 0.1875 0.1875] Sistema de interacción
  ;;[0.349 0.2341 0.1177 1 14] Cuando el PJ deje de estar encima del obj se CIERRA
  ;;[0.3125 0.3125 0.3125 1 14] No deja que pueda seguir el curso de los nodos a menos que...
  (Utilities|FlowControl|Gate true) ; enters at Close
)

(fn ConstructionScript)