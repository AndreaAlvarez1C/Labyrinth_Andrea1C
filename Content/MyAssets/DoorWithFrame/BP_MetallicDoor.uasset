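; Metallic door with frame that swings open and closed each time its OpenCloseDoor event is called.
; BeginPlay chooses the swing direction from the InvertDirection flag, giving a quarter turn either way.
; A FlipFlop alternately plays and reverses the DoorRotation timeline, whose Alpha interpolates the door mesh's relative rotation between closed and open.
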(event Custom|OpenCloseDoor
  ;[0.03125 0.03125 0.03125] Abrir/Cerrar la puerta
  ;;[0.2708 0.2708 0.2708 1 14] Para poder abrir y cerrar la puerta
  (Utilities|FlowControl|FlipFlop
    (:A
      ;;[0.4688 0.4436 0.249 1 14] La variación de ALPHA en 0.7s
      (bind _alpha (Timeline|DoorRotation Play)
        (:Update
          (Transformation|SetRelativeRotation (Variables|Default|GetDoor_Door_GEO) (Math|Rotator|Lerp(Rotator) "0, 0, 0" (Variables|Default|GetDoorDirection) _alpha) false false))))
    (:B
      (Timeline|DoorRotation Reverse))))

(event EventBeginPlay
  ;[0.1875 0.1875 0.1875] Sistema de interacción
  ;[0.125 0.07878 0.07878 1 14] Rotación interna/externa de la puerta
  (if (Variables|Default|GetInvertDirection)
    (Variables|Default|SetDoorDirection "0.000000,90.000000,0.000000")
    (else
      (Variables|Default|SetDoorDirection "0.000000,-90.000000,0.000000"))))

(event EventTick
  (params (DeltaSeconds :type Float%20%28single-precision%29)))

(fn ConstructionScript)